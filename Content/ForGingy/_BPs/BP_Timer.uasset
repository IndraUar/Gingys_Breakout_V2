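; BP_Timer is a minutes-and-seconds countdown that ends the game when it reaches zero.
; Tick runs through a one-second Delay, then decrements TimerSeconds, rolling over to 59 and reducing TimerMinutes as needed.
; At zero it shows the mouse cursor, sets cinematic mode to lock movement and turning, and adds a GameOver_ widget to the viewport.
; Nothing stops the Tick afterwards, so this end branch repeats each second.
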(event EventTick
  (params (DeltaSeconds :type Float%20%28single-precision%29))
  (bind _returnvalue (Game|GetPlayerController 0))
  ;[1 1 1] CountDown
  (Utilities|FlowControl|Delay 1.0)
  (if (== (Variables|Default|GetTimerSeconds) 0)
    (if (== (Variables|Default|GetTimerMinutes) 0)
      (Variables|/Script/Engine.PlayerController|SetbShowMouseCursor _returnvalue true)
      (Class|PlayerController|SetCinematicMode _returnvalue true true true true true)
      (bind _returnvalue_2 (UserInterface|CreateWidget "/Game/GingyBreakout/UI/GameEnd/GameOver_.GameOver__C" _returnvalue))
      (UserInterface|Viewport|AddtoViewport _returnvalue_2 0)
      (else
        (Variables|Default|SetTimerSeconds 59)
        (Variables|Default|SetTimerMinutes (- (Variables|Default|GetTimerMinutes) 1))))
    (else
      (Variables|Default|SetTimerSeconds (- (Variables|Default|GetTimerSeconds) 1)))))

(fn ConstructionScript)